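; Survival game mode Blueprint that handles boss-battle music and the wave UI for a wave-based survival match.
; It listens to the game mode state change event, showing countdown or plain wave banners as waves wait, spawn and complete.
; The final wave sets a spawn delay and adds a "Last Wave" banner.
; Victory or player death clears widgets, fades the camera out, then async-loads the win or lose screen.
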(event `self.ReceiveBeginPlay`
  (`GameplayStatics.SpawnSound2D` "/Game/Assets/Sounds/Music/Dungeons_EndBossBattle.Dungeons_EndBossBattle" 1.0 1.0 0.0 null)
  (add `self.OnSurvialGameModeStateChanged` (delegate `OnSurvialGameModeStateChanged_Event`)))

(event `OnSurvialGameModeStateChanged_Event` :!signature `self.OnSurvialGameModeStateChanged`
  (params (CurrentState :type "ESurvialGameModeState Enum" :default "WaitSpawnNewWave"))
  (bind _returnvalue (`GameplayStatics.GetPlayerCameraManager` 0))
  (bind _returnvalue_2 (`GameplayStatics.GetPlayerCameraManager` 0))
  (switch `ESurvialGameModeState` CurrentState
    (:`WaitSpawnNewWave`
      (`self.Create Wave Widget Width Count Down` "New Wave Coming In" (`self.SpawnNewWaveWaitTime`)))
    (:`SpawningNewWave`
      (`self.Create Wave Widget No CountDown` (`|FormatText` "Wave {CurrentWaveCount} " (`self.CurrentWaveCount`)))
      (if (== (`self.TotalWavesToSpawn`) (`self.CurrentWaveCount`))
        (set `self.SpawnEnemiesDelayTime` 4.0)
        (`KismetSystemLibrary.Delay` 2.0)
        (`self.Create Wave Widget No CountDown` "Last Wave")))
    (:`WaveCompleted`
      (`self.Create Wave Widget Width Count Down` (`|FormatText` "Wave {CurrentWaveCount}  Complete" (`self.CurrentWaveCount`)) (`self.WaveCompleteWaitTime`)))
    (:`AllWavesDone`
      (`KismetSystemLibrary.Delay` 1.5)
      (`WidgetLayoutLibrary.RemoveAllWidgets`)
      (`/Engine/EditorBlueprintResources/StandardMacros.IsValid` _returnvalue_2
        (:`Is Valid`
          (`PlayerCameraManager.StartCameraFade` :`self` _returnvalue_2 :`ToAlpha` 1.0 :`Duration` 3.0 :`bHoldWhenFinished` true)
          (`KismetSystemLibrary.Delay` 3.0)
          (bind _class (`|LoadAssetClass` "/Game/Widgets/GameModeWidgets/WBP_WinScreen.WBP_WinScreen_C")
            (:`Completed`
              (bind _asuser_widget (castclass `UserWidget` _class))
              (bind _returnvalue_3 (`|CreateWidget` _asuser_widget))
              (`UserWidget.AddToViewport` _returnvalue_3 0))))))
    (:`PlayerDied`
      (`WidgetLayoutLibrary.RemoveAllWidgets`)
      (`/Engine/EditorBlueprintResources/StandardMacros.IsValid` _returnvalue
        (:`Is Valid`
          (`PlayerCameraManager.StartCameraFade` :`self` _returnvalue :`ToAlpha` 1.0 :`Duration` 2.0 :`bHoldWhenFinished` true)
          (`KismetSystemLibrary.Delay` 2.0)
          (bind _class_2 (`|LoadAssetClass` "/Game/Widgets/GameModeWidgets/WBP_LoseScreen.WBP_LoseScreen_C")
            (:`Completed`
              (bind _asuser_widget_2 (castclass `UserWidget` _class_2))
              (bind _returnvalue_4 (`|CreateWidget` _asuser_widget_2))
              (`UserWidget.AddToViewport` _returnvalue_4 0))))))))

(fn `Create Wave Widget No CountDown`
  (params (`Text Content To Display` :type Text))
  (bind _returnvalue (`|CreateWidget` "/Game/Widgets/GameModeWidgets/WBP_WaveTextNoCountDown.WBP_WaveTextNoCountDown_C"))
  (`UserWidget.AddToViewport` _returnvalue 0)
  (`TextBlock.SetText` (`/Game/Widgets/GameModeWidgets/WBP_WaveTextNoCountDown.TextBlock_WaveText` _returnvalue) (`local.Text Content To Display`)))

(fn `Create Wave Widget Width Count Down`
  (params (TextContentToDisplay :type Text) (InTotalCountDownTime :type "Float (double-precision)"))
  (bind _returnvalue (`|CreateWidget` "/Game/Widgets/GameModeWidgets/WBP_WaveTextWithCountDown.WBP_WaveTextWithCountDown_C"))
  (`UserWidget.AddToViewport` _returnvalue 0)
  (`TextBlock.SetText` (`/Game/Widgets/GameModeWidgets/WBP_WaveTextWithCountDown.TextBlock_WaveText` _returnvalue) (`local.TextContentToDisplay`))
  (`/Game/Widgets/GameModeWidgets/WBP_WaveTextWithCountDown.StartCountDown` _returnvalue (`local.InTotalCountDownTime`)))

(fn `UserConstructionScript`)