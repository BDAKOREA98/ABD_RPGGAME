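; Survival game mode Blueprint that announces each upcoming enemy-free wave wait with an on-screen countdown.
; On BeginPlay it binds to its state-changed dispatcher and reacts only to the Wait Spawn New Wave state.
; That state calls a helper that creates a WBP_WaveTextWithCountDown widget, sets text naming the current wave and starts a countdown lasting the spawn wait time.
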(event `self.ReceiveBeginPlay`
  (add `self.OnSurvialGameModeStateChanged` (delegate `OnSurvialGameModeStateChanged_Event`)))

(event `OnSurvialGameModeStateChanged_Event` :!signature `self.OnSurvialGameModeStateChanged`
  (params (CurrentState :type "ESurvialGameModeState Enum" :default "WaitSpawnNewWave"))
  (switch `ESurvialGameModeState` CurrentState
    (:`WaitSpawnNewWave`
      (`self.Create Wave Widget Width Count Down` (`|FormatText` "Wave {CurrentWaveCount} Coming In" (`self.CurrentWaveCount`)) (`self.SpawnNewWaveWaitTime`)))))

(fn `Create Wave Widget Width Count Down`
  (params (TextContentToDisplay :type Text) (InTotalCountDownTime :type "Float (double-precision)"))
  (bind _returnvalue (`|CreateWidget` "/Game/Widgets/GameModeWidgets/WBP_WaveTextWithCountDown.WBP_WaveTextWithCountDown_C"))
  (`UserWidget.AddToViewport` _returnvalue 0)
  (`TextBlock.SetText` (`/Game/Widgets/GameModeWidgets/WBP_WaveTextWithCountDown.TextBlock_WaveText` _returnvalue) (`local.TextContentToDisplay`))
  (`/Game/Widgets/GameModeWidgets/WBP_WaveTextWithCountDown.StartCountDown` _returnvalue (`local.InTotalCountDownTime`)))

(fn `UserConstructionScript`)