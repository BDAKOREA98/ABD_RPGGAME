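; Base enemy Blueprint that handles the visual entrance and death of enemies.
; On BeginPlay, a reversed timeline un-dissolves the mesh and equipped weapon while a random entry montage plays.
; On death, it freezes animation, disables capsule collision, removes widgets, and async-loads a Niagara effect tinted by the material's dissolve edge color.
; A timeline dissolves mesh and weapon, then the weapon is destroyed, the SpawnStone ability is triggered and the actor is destroyed.
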(event `self.ReceiveBeginPlay`
  (bind _entrymontagetopley (`self.EntryMontageToPley`))
  (bind _returnvalue (`C_PawnCombatComponent.GetCreatureCurrentEquippedWeapon` (`self.EnemyCombatComponent`)))
  (`|ExecutionSequence`
    (:`then_0`
      (`TimelineComponent.SetPlayRate` (`self.EntryRestoreTimeline`) (/ 1.0 (`self.TotalEntryRestoreTime`)))
      (bind (_direction _normalizedfloattrack) (`Timeline|EntryRestoreTimeline` :!via `ReverseFromEnd`)
        (:`Update`
          (`MeshComponent.SetScalarParameterValueOnMaterials` (`self.Mesh`) "DissolveAmount" _normalizedfloattrack)
          (`/Engine/EditorBlueprintResources/StandardMacros.IsValid` _returnvalue
            (:`Is Valid`
              (`MeshComponent.SetScalarParameterValueOnMaterials` (`WarriorWeaponBase.WeaponMesh` _returnvalue) "DissolveAmount" _normalizedfloattrack))))))
    (:`then_1`
      (if (`KismetArrayLibrary.Array_IsNotEmpty` _entrymontagetopley)
        (`self.PlayAnimMontage` (`KismetArrayLibrary.Array_Random` _entrymontagetopley))))))

(event `/Game/Blueprint/Enemy/BPI_EnemyDeath.OnEnemyDied`
  (params (DissolveNiagaraSysten :type "NiagaraSystem Soft Object Reference"))
  (bind _mesh (`self.Mesh`))
  (bind _returnvalue (`C_PawnCombatComponent.GetCreatureCurrentEquippedWeapon` (`self.EnemyCombatComponent`)))
  (bind _returnvalue_2 (`C_PawnCombatComponent.GetCreatureCurrentEquippedWeapon` (`self.EnemyCombatComponent`)))
  (`|ExecutionSequence`
    (:`then_0`
      (set `SkeletalMeshComponent.bPauseAnims` true (`self.Mesh`))
      (`PrimitiveComponent.SetCollisionEnabled` (`self.CapsuleComponent`) "NoCollision"))
    (:`then_1`
      (`C_EnemyUIComponent.RemoveEnemyDrawnWidgetsIfAny` (`self.EnemyUIComponent`)))
    (:`then_2`
      (bind _object (`|LoadAsset` DissolveNiagaraSysten)
        (:`Completed`
          (bind _asniagara_system (cast `NiagaraSystem` _object))
          (bind _returnvalue_3 (`NiagaraFunctionLibrary.SpawnSystemAttached` _asniagara_system (`self.Mesh`) "None" (0.0 0.0 0.0) (struct) "KeepRelativeOffset"))
          (bind _returnvalue_4 (`PrimitiveComponent.CreateDynamicMaterialInstance` _mesh 0 (`PrimitiveComponent.GetMaterial` _mesh 0) "None"))
          (bind _returnvalue_5 (`MaterialInstanceDynamic.K2_GetVectorParameterValue` _returnvalue_4 "DissolveEdgeColor"))
          (`NiagaraComponent.SetNiagaraVariableLinearColor` _returnvalue_3 "DissolveParticleColor" _returnvalue_5)
          (`TimelineComponent.SetPlayRate` (`self.Dissove Timeline`) (/ 1.0 (`self.TotalDissolveTime`)))
          (bind (_direction _normalizedfloattrack) (`Timeline|Dissove Timeline` :!via `PlayFromStart`)
            (:`Update`
              (`MeshComponent.SetScalarParameterValueOnMaterials` (`self.Mesh`) "DissolveAmount" _normalizedfloattrack)
              (`/Engine/EditorBlueprintResources/StandardMacros.IsValid` _returnvalue_2
                (:`Is Valid`
                  (`MeshComponent.SetScalarParameterValueOnMaterials` (`WarriorWeaponBase.WeaponMesh` _returnvalue_2) "DissolveAmount" _normalizedfloattrack))))
            (:`Finished`
              (`/Engine/EditorBlueprintResources/StandardMacros.IsValid` _returnvalue
                (:`Is Valid`
                  (`self.K2_DestroyActor` _returnvalue))
                (:`Is Not Valid`
                  _))
              (`C_WarriorAbilityComponent.TryActivateAbilityByTag` (`self.WarriorAbilityComponent`) (struct :`TagName` "Enemy.Ability.SpawnStone"))
              (`KismetSystemLibrary.Delay` 0.5)
              (`self.K2_DestroyActor`))))))))

(fn `UserConstructionScript`)